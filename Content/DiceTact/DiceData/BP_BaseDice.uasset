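; Base Blueprint for combat dice that collide with each other, damage what they hit and show their resolve effect.
; Mesh hits trigger dice-to-dice impact logic and FX, and deal one damage to each damageable actor only once.
; On initialization it async-loads FX and material from its resolve definition, while a widget displays its number.
; Bounces puff smoke, fracturing briefly slows time, and settling or finishing resolution releases camera focus.
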(event `self.ReceiveBeginPlay`
  ; OLD way for the camera to focus on the dice
  (`parent.ReceiveBeginPlay`)
  (bind _aswbp_dice_number_widget (cast `/Game/DiceTact/UI/Widgets/WBP_DiceNumberWidget` (`WidgetComponent.GetWidget` (`self.Widget`))))
  (`/Game/DiceTact/UI/Widgets/WBP_DiceNumberWidget.SetDice` _aswbp_dice_number_widget self))

(event `self.OnBeforeDiceDestroyed`
  (`ActorComponent.K2_DestroyComponent` (`self.Widget`)))

(event `self.DiceMesh.OnComponentHit`
  (params (HitComponent :type "PrimitiveComponent Object Reference") (OtherActor :type "Actor Object Reference") (OtherComp :type "PrimitiveComponent Object Reference") (NormalImpulse :type "Vector Structure") (Hit :type "HitResult Structure (by ref)"))
  (`|ExecutionSequence`
    (:`then_0`
      (bind _asdtdice (cast `DTDice` OtherActor))
      (`self.OnDiceHit` _asdtdice Hit)
      (`NiagaraFunctionLibrary.SpawnSystemAtLocation` "/Game/DiceTact/Effects/Impact/NS_Impact.NS_Impact" (`self.K2_GetActorLocation`)))
    (:`then_2`
      (bind _asdtdamageable (cast `DTDamageable` OtherActor))
      (if (not (`BlueprintMapLibrary.Map_Contains` (`self.EnemyHit`) OtherActor))
        (`DTDamageable.TakeDamage` _asdtdamageable self 1)
        (`BlueprintMapLibrary.Map_Add` (`self.EnemyHit`) OtherActor)))))

(event `DEBUG_ResolveDice`
  (`self.ResolveDice`))

(event `self.OnBounceGround`
  (params (Location :type "Vector Structure"))
  (`NiagaraFunctionLibrary.SpawnSystemAtLocation` "/Game/DiceTact/Effects/DiceEffects/ActiveEffect/Dust/NS_SmokePuffs.NS_SmokePuffs" (+ Location (0.0 0.0 10.0))))

(event `self.OnInitializationFinished`
  (bind _dicemesh (`self.DiceMesh`))
  (bind _returnvalue (`DTDiceResolveDefinition.GetResolveFX` (`self.ResolveDefinition`)))
  (bind _returnvalue_2 (`DTDiceResolveDefinition.GetResolveMaterial` (`self.ResolveDefinition`)))
  (bind _output (`|ConvertAsset` _returnvalue_2))
  ;[0 0 0 0.5] On Initilisation finished
  (`|ExecutionSequence`
    (:`then_0`
      (if (`KismetSystemLibrary.IsValidSoftObjectReference` _returnvalue)
        (`|LoadAsset` _returnvalue
          (:`Completed`
            (`NiagaraComponent.SetAsset` (`self.ResolveFX`) (`|ConvertAsset` _returnvalue) true)))))
    (:`then_1`
      (if (`KismetSystemLibrary.IsValidSoftObjectReference` _returnvalue_2)
        (`|LoadAsset` _returnvalue_2
          (:`Completed`
            (`PrimitiveComponent.SetMaterialByName` _dicemesh "phongE2" _output)
            (`PrimitiveComponent.SetMaterialByName` _dicemesh "translucent" _output)))))))

(event `self.OnDiceSettled`
  (`DTCombatBridgeSubsystem.UnregisterNewFocus` (subsystem `DTCombatBridgeSubsystem`) self)
  (`ActorComponent.Deactivate` (`self.ResolveFX`)))

(event `self.OnResolutionStarted`)

(event `self.OnResolutionFinished`
  (`DTCombatBridgeSubsystem.UnregisterNewFocus` (subsystem `DTCombatBridgeSubsystem`) self))

(event `self.OnDiceFractured`
  (params (MyTypeSide :type "EDiceType Enum" :default "four") (DiceToSpawn :type "Array of EDiceType Enum (by ref)" :default _))
  (`DTTimeControllerSubsystem.RequestTimeStop` (subsystem `DTTimeControllerSubsystem`) 0.2 0.05 0.05 0.05 2.0))

(fn `UserConstructionScript`)