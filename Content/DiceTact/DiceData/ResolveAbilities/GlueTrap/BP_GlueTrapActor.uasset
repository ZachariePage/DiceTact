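; BP_GlueTrapActor is a glue trap that puts a Gameplay Effect on enemy units while they overlap it.
; Overlap begin applies TrapEffect through the unit's Ability System Component and maps the unit to the effect handle in ActiveEffects.
; Overlap end removes the effect by that handle but keeps the map entry.
; CleanupTrap only removes map entries while looping, leaving applied effects untouched, and BeginPlay briefly draws a debug radius sphere.
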(event `self.ReceiveBeginPlay`
  (`KismetSystemLibrary.DrawDebugSphere` (`self.K2_GetActorLocation`) (`self.TrapRadius`) 12 (struct :`R` 1.0 :`G` 1.0 :`B` 1.0 :`A` 1.0) 3.0 1.0))

(event `self.ReceiveActorBeginOverlap`
  (params (OtherActor :type "Actor Object Reference"))
  (bind _asenemy_unit (cast `EnemyUnit` OtherActor))
  (bind _returnvalue (`AbilitySystemComponent.BP_ApplyGameplayEffectToSelf` :`self` (`EnemyUnit.AbilitySystemComponent` _asenemy_unit) :`GameplayEffectClass` (`self.TrapEffect`)))
  (`BlueprintMapLibrary.Map_Add` (`self.ActiveEffects`) _asenemy_unit _returnvalue))

(event `self.ReceiveActorEndOverlap`
  (params (OtherActor :type "Actor Object Reference"))
  (bind _asenemy_unit (cast `EnemyUnit` OtherActor))
  (bind (_value _returnvalue) (`BlueprintMapLibrary.Map_Find` (`self.ActiveEffects`) _asenemy_unit))
  (if _returnvalue
    (`AbilitySystemComponent.RemoveActiveGameplayEffect` (`EnemyUnit.AbilitySystemComponent` _asenemy_unit) _value -1)))

(event `self.CleanupTrap`
  (bind _activeeffects (`self.ActiveEffects`))
  (bind _keypin (`|MapForEach` _activeeffects)
    (:`then`
      (`BlueprintMapLibrary.Map_Remove` _activeeffects _keypin))))

(fn `UserConstructionScript`)