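; Cage gameplay ability that boxes in its owner with four BP_CageWall actors.
; On activation it commits, then calls one spawn function per side, each offsetting from the owner's location along world X or Y, regardless of facing.
; Wall length comes from AbilityData and grows linearly with ability level, setting both each wall's offset and its InitializeWall size.
; The ability never calls EndAbility.
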(event `self.K2_ActivateAbility`
  (`self.K2_CommitAbility`)
  ; I KNOW IT WOULD BE BETTER IN A FOR LOOP I KNOW
  (`self.SpawnFrontWall`)
  (`self.SpawnRightWall`)
  (`self.SpawnLeftWall`)
  (`self.SpawnBehindWall`))

(fn `SpawnBehindWall`
  (bind _returnvalue (`|SpawnActorFromClass` "/Game/DiceTact/DiceData/ResolveAbilities/Cage/BP_CageWall.BP_CageWall_C" (`KismetMathLibrary.Conv_VectorToTransform` (- (`Actor.K2_GetActorLocation` (`.OwnerActor` (break `GameplayAbilityActorInfo` (`self.GetActorInfo`)))) (`KismetMathLibrary.MakeVector` (* (`KismetMathLibrary.SafeDivide` (+ (* (`DTCageData.additionalWallSize` (`self.AbilityData`)) (`self.GetAbilityLevel`)) (`DTCageData.defaultSizeOfWall` (`self.AbilityData`))) 2.0) 200.0)))) "Undefined" "MultiplyWithRoot" null null))
  (`/Game/DiceTact/DiceData/ResolveAbilities/Cage/BP_CageWall.InitializeWall` _returnvalue (`KismetMathLibrary.MakeVector` 1.0 (+ (* (`DTCageData.additionalWallSize` (`self.AbilityData`)) (`self.GetAbilityLevel`)) (`DTCageData.defaultSizeOfWall` (`self.AbilityData`))) 1.0)))

(fn `SpawnFrontWall`
  (locals (NewLocalVar :type "Float (double-precision)"))
  (bind _returnvalue (`|SpawnActorFromClass` "/Game/DiceTact/DiceData/ResolveAbilities/Cage/BP_CageWall.BP_CageWall_C" (`KismetMathLibrary.Conv_VectorToTransform` (+ (`Actor.K2_GetActorLocation` (`.OwnerActor` (break `GameplayAbilityActorInfo` (`self.GetActorInfo`)))) (`KismetMathLibrary.MakeVector` (* (`KismetMathLibrary.SafeDivide` (+ (* (`DTCageData.additionalWallSize` (`self.AbilityData`)) (`self.GetAbilityLevel`)) (`DTCageData.defaultSizeOfWall` (`self.AbilityData`))) 2.0) 200.0)))) "Undefined" "MultiplyWithRoot" null null))
  (`/Game/DiceTact/DiceData/ResolveAbilities/Cage/BP_CageWall.InitializeWall` _returnvalue (`KismetMathLibrary.MakeVector` 1.0 (+ (* (`DTCageData.additionalWallSize` (`self.AbilityData`)) (`self.GetAbilityLevel`)) (`DTCageData.defaultSizeOfWall` (`self.AbilityData`))) 1.0)))

(fn `SpawnLeftWall`
  (bind _returnvalue (`|SpawnActorFromClass` "/Game/DiceTact/DiceData/ResolveAbilities/Cage/BP_CageWall.BP_CageWall_C" (`KismetMathLibrary.Conv_VectorToTransform` (- (`Actor.K2_GetActorLocation` (`.OwnerActor` (break `GameplayAbilityActorInfo` (`self.GetActorInfo`)))) (`KismetMathLibrary.MakeVector` 0.0 (* (`KismetMathLibrary.SafeDivide` (+ (* (`DTCageData.additionalWallSize` (`self.AbilityData`)) (`self.GetAbilityLevel`)) (`DTCageData.defaultSizeOfWall` (`self.AbilityData`))) 2.0) 200.0)))) "Undefined" "MultiplyWithRoot" null null))
  (`/Game/DiceTact/DiceData/ResolveAbilities/Cage/BP_CageWall.InitializeWall` _returnvalue (`KismetMathLibrary.MakeVector` (+ (* (`DTCageData.additionalWallSize` (`self.AbilityData`)) (`self.GetAbilityLevel`)) (`DTCageData.defaultSizeOfWall` (`self.AbilityData`))) 1.0 1.0)))

(fn `SpawnRightWall`
  (bind _returnvalue (`|SpawnActorFromClass` "/Game/DiceTact/DiceData/ResolveAbilities/Cage/BP_CageWall.BP_CageWall_C" (`KismetMathLibrary.Conv_VectorToTransform` (+ (`Actor.K2_GetActorLocation` (`.OwnerActor` (break `GameplayAbilityActorInfo` (`self.GetActorInfo`)))) (`KismetMathLibrary.MakeVector` 0.0 (* (`KismetMathLibrary.SafeDivide` (+ (* (`DTCageData.additionalWallSize` (`self.AbilityData`)) (`self.GetAbilityLevel`)) (`DTCageData.defaultSizeOfWall` (`self.AbilityData`))) 2.0) 200.0)))) "Undefined" "MultiplyWithRoot" null null))
  (`/Game/DiceTact/DiceData/ResolveAbilities/Cage/BP_CageWall.InitializeWall` _returnvalue (`KismetMathLibrary.MakeVector` (+ (* (`DTCageData.additionalWallSize` (`self.AbilityData`)) (`self.GetAbilityLevel`)) (`DTCageData.defaultSizeOfWall` (`self.AbilityData`))) 1.0 1.0)))