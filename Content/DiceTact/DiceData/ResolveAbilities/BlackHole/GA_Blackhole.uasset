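; Black Hole gameplay ability, one of the dice resolve abilities, that spawns a black hole visual at the owning actor's location.
; On activation it commits, computes a radius from its data's base plus a per-level addition, and draws a debug sphere at that size.
; The Niagara effect's ScaleMultiplier is set from the same radius.
; It applies no pull or damage and never calls EndAbility in this graph.
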(event `self.K2_ActivateAbility`
  (bind _data (`self.data`))
  (bind _returnvalue (`Actor.K2_GetActorLocation` (`.OwnerActor` (break `GameplayAbilityActorInfo` (`self.GetActorInfo`)))))
  (`self.K2_CommitAbility`)
  (`KismetSystemLibrary.DrawDebugSphere` _returnvalue (+ (`DTBlackHoleData.BaseRadius` (`self.data`)) (* (`DTBlackHoleData.AdditionalRadius` (`self.data`)) (`self.GetAbilityLevel`))) 12 (struct :`R` 1.0 :`G` 1.0 :`B` 1.0 :`A` 1.0) 3.0 1.0)
  (bind _returnvalue_2 (`NiagaraFunctionLibrary.SpawnSystemAtLocation` "/Game/DiceTact/Effects/DiceEffects/ActiveEffect/BlackHole/Sub/NS_BlackHole.NS_BlackHole" _returnvalue))
  (`NiagaraComponent.SetNiagaraVariableFloat` _returnvalue_2 "ScaleMultiplier" (/ (+ (`DTBlackHoleData.BaseRadius` _data) (* (`DTBlackHoleData.AdditionalRadius` _data) (`self.GetAbilityLevel`))) 250.0)))

(event `self.K2_OnEndAbility`
  (params (bWasCancelled :type Boolean)))