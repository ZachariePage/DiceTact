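; BP_Meteor is a meteor projectile that deals area damage when its mesh hits something.
; On hit it sphere-overlaps the affected object types within its explosion radius and deals one damage to each Damageable found.
; The destroy call sits inside that loop, so the meteor is only destroyed when a Damageable is processed.
; OnExplosion currently just draws a debug sphere showing the blast area.
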(event `self.MeteorMesh.OnComponentHit`
  (params (HitComponent :type "PrimitiveComponent Object Reference") (OtherActor :type "Actor Object Reference") (OtherComp :type "PrimitiveComponent Object Reference") (NormalImpulse :type "Vector Structure") (Hit :type "HitResult Structure (by ref)"))
  (`self.OnExplosion` (`self.ExplosionRadius`) (`self.K2_GetActorLocation`))
  (bind _outactors (`KismetSystemLibrary.SphereOverlapActors` (`self.K2_GetActorLocation`) (`self.ExplosionRadius`) (`self.AffectedType`)))
  (for _array_element _outactors
    (bind _asdamageable (cast `Damageable` _array_element))
    (`Damageable.TakeDamage` _asdamageable self 1)
    (`self.K2_DestroyActor`)))

(event `OnExplosion`
  (params (ExplosionSize :type "Float (double-precision)") (ExplosionLocation :type "Vector Structure"))
  (`KismetSystemLibrary.DrawDebugSphere` ExplosionLocation ExplosionSize 12 (struct :`R` 0.034634 :`G` 0.048829 :`B` 1.0 :`A` 1.0) 2.0 3.0))

(fn `UserConstructionScript`)