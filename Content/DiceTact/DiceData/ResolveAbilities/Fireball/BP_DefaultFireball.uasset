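; BP_DefaultFireball is a projectile actor, the default fireball of a resolve ability, moved by a ProjectileMovement component on its collider and drawn with Niagara.
; An Impulse event adds force directly to its velocity.
; Overlaps and hits flag it for delayed destruction by a Tick countdown, and hits also deal fixed damage to Damageable actors.
; The collider is hidden only in shipping builds.
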(event `self.ReceiveBeginPlay`
  (bind _collider (`self.Collider`))
  (`parent.ReceiveBeginPlay`)
  (`SceneComponent.SetHiddenInGame` _collider (`JUESystemStatics.IsInBuildShipping`) false)
  (`MovementComponent.SetUpdatedComponent` (`self.ProjectileMovement`) _collider)
  (`NiagaraComponent.SetAsset` (`self.Niagara`) (`self.NiagaraSystem`) true))

(event `Impulse`
  (params (Force :type "Vector Structure"))
  (bind _projectilemovement (`self.ProjectileMovement`))
  (set `MovementComponent.Velocity` (+ Force (`MovementComponent.Velocity` _projectilemovement)) _projectilemovement))

(event `self.ReceiveTick`
  (params (DeltaSeconds :type "Float (single-precision)"))
  (if (`self.DestroyPending`)
    (set `self.Timer` (- (`self.Timer`) DeltaSeconds))
    (if (< (`self.Timer`) 0.0)
      (`self.K2_DestroyActor`))))

(event `self.Sphere.OnComponentBeginOverlap`
  (params (OverlappedComponent :type "PrimitiveComponent Object Reference") (OtherActor :type "Actor Object Reference") (OtherComp :type "PrimitiveComponent Object Reference") (OtherBodyIndex :type Integer) (bFromSweep :type Boolean) (SweepResult :type "HitResult Structure (by ref)"))
  (set `self.DestroyPending` true))

(event `self.Sphere.OnComponentHit`
  (params (HitComponent :type "PrimitiveComponent Object Reference") (OtherActor :type "Actor Object Reference") (OtherComp :type "PrimitiveComponent Object Reference") (NormalImpulse :type "Vector Structure") (Hit :type "HitResult Structure (by ref)"))
  (set `self.DestroyPending` true)
  (bind _asdamageable (cast `Damageable` OtherActor))
  (`Damageable.TakeDamage` _asdamageable self 5))

(fn `UserConstructionScript`)