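; Magic missile projectile actor that deals explosive area damage to enemies when its mesh hits something.
; The hit runs a sphere overlap at the explosion radius, temporarily filtered to BP_BaseEnemyCharacter so the cart is spared.
; Each overlapped DTDamageable takes one damage.
; The OnExplosion debug sphere and actor destruction sit inside that loop, so neither happens when no damageable enemy is in range.
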(event `OnExplosion`
  (params (ExplosionLocation :type "Vector Structure") (ExplosionSize :type "Float (double-precision)"))
  (`KismetSystemLibrary.DrawDebugSphere` ExplosionLocation ExplosionSize 12 (struct :`G` 0.052323 :`B` 1.0 :`A` 1.0) 2.0 2.0))

(event `self.MagicMissileMesh.OnComponentHit`
  (params (HitComponent :type "PrimitiveComponent Object Reference") (OtherActor :type "Actor Object Reference") (OtherComp :type "PrimitiveComponent Object Reference") (NormalImpulse :type "Vector Structure") (Hit :type "HitResult Structure (by ref)"))
  ; Filtre Temporaire pour ne pas frapper cart avec explosion
  (bind _outactors (`KismetSystemLibrary.SphereOverlapActors` (`self.K2_GetActorLocation`) (`self.ExplosionRadius`) (`self.AffectedTypes`) "/Game/DiceTact/Characters/Enemies/BP_BaseEnemyCharacter.BP_BaseEnemyCharacter_C"))
  (for _array_element _outactors
    (bind _asdtdamageable (cast `DTDamageable` _array_element))
    (`self.OnExplosion` (`self.K2_GetActorLocation`) (`self.ExplosionRadius`))
    (`DTDamageable.TakeDamage` _asdtdamageable self 1)
    (`self.K2_DestroyActor`)))

(fn `UserConstructionScript`)