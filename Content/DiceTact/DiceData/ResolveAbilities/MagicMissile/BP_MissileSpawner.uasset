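; Spawner actor for the Magic Missile ability that creates a BP_MagicMissile on BeginPlay and flies it to a homing target.
; SetHomingTarget builds a spline from a synchronous navigation path between the owner and a valid target, then launches.
; A timeline scaled by TimeToTarget moves the missile along the spline, destroying the spawner if the missile becomes invalid.
; The path-update handler is empty and the fallback location never triggers a launch.
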(event `self.ReceiveBeginPlay`
  (bind _returnvalue (`|SpawnActorFromClass` "/Game/DiceTact/DiceData/ResolveAbilities/MagicMissile/BP_MagicMissile.BP_MagicMissile_C" (`self.GetTransform`) "AdjustIfPossibleButAlwaysSpawn" "MultiplyWithRoot" (`self.GetOwner` self) null))
  (set `self.SpawnedMagicMissile` _returnvalue)
  (`KismetSystemLibrary.DrawDebugSphere` (`self.K2_GetActorLocation`) 50.0 12 (struct :`R` 0.562314 :`G` 0.013793 :`B` 1.0 :`A` 1.0) 2.0))

(event `LaunchMissile`
  (`TimelineComponent.SetPlayRate` (`self.T_Move`) (/ 1.0 (`self.TimeToTarget`)))
  (bind (_direction _move_track) (`Timeline|T_Move`)
    (:`Update`
      (if (`KismetSystemLibrary.IsValid` (`self.SpawnedMagicMissile`))
        (`self.K2_SetActorLocation` (`self.SpawnedMagicMissile`) (`SplineComponent.GetLocationAtDistanceAlongSpline` (`self.Spline`) (`KismetMathLibrary.Lerp` 0.0 (`SplineComponent.GetSplineLength` (`self.Spline`)) _move_track) "World") false false)
        (else
          (`self.K2_DestroyActor`))))))

(event `UpdatePath`
  (params (AffectedPath :type "NavigationPath Object Reference") (PathEvent :type "ENavPathEvent Enum" :default "Cleared")))

(event `self.SetHomingTarget`
  (params (InTarget :type "Actor Object Reference") (InFallbackTargetLocation :type "Vector Structure"))
  (set `DTMagicMissileActor.HomingTarget` InTarget (`self.SpawnedMagicMissile`))
  (set `self.GoalLocation` InFallbackTargetLocation)
  (if (`KismetSystemLibrary.IsValid` InTarget)
    (set `self.GoalLocation` (+ (`self.K2_GetActorLocation` InTarget) (`KismetMathLibrary.MakeVector` 0.0 0.0 (`DTMagicMissileActor.TargetZOffset` (`self.SpawnedMagicMissile`)))))
    (bind _returnvalue (`NavigationSystemV1.FindPathToActorSynchronously` (`self.K2_GetActorLocation` (`self.GetOwner`)) (`DTMagicMissileActor.HomingTarget` (`self.SpawnedMagicMissile`)) 20.0 null null))
    (add `NavigationPath.PathUpdatedNotifier` _returnvalue (delegate `UpdatePath`))
    (`SplineComponent.SetSplinePoints` (`self.Spline`) (`NavigationPath.PathPoints` _returnvalue) "World" true)
    (`self.LaunchMissile`)))

(fn `UserConstructionScript`)