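; BP_Chariot is a turn-based character Blueprint for the Chariot in DiceTact, with a health component and a widget health bar.
; On BeginPlay it runs the parent logic, caches the health bar widget, and initializes it from the HealthComponent one frame later.
; Health changes drive animated bar updates.
; Its Turn event takes no action beyond waiting briefly and signaling that the turn has finished.
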(event `self.ReceiveBeginPlay`
  (bind _healthcomponent (`self.HealthComponent`))
  (`parent.ReceiveBeginPlay`)
  (bind _aswbp_health_bar (cast `/Game/DiceTact/UI/Widgets/Combat/WBP_HealthBar` (`WidgetComponent.GetWidget` (`self.HealthWidget`))))
  (bind _output_get (set `self.HealthBarWidget` _aswbp_health_bar))
  (`KismetSystemLibrary.DelayUntilNextFrame`)
  (`/Game/DiceTact/UI/Widgets/Combat/WBP_HealthBar.InitializeHealthBar` _output_get (`HealthComponent.MaxHealth` _healthcomponent) (`HealthComponent.CurrentHealth` _healthcomponent)))

(event `self.ReceiveTurn`
  (`KismetSystemLibrary.Delay` 0.5)
  (`self.OnTurnFinished`))

(event `self.HealthComponent.OnCurrentHealthChanged`
  (params (OldValue :type Integer) (NewValue :type Integer))
  (bind _healthbarwidget (`self.HealthBarWidget`))
  (`/Engine/EditorBlueprintResources/StandardMacros.IsValid` _healthbarwidget
    (:`Is Valid`
      (`/Game/DiceTact/UI/Widgets/Combat/WBP_HealthBar.UpdateHealth` _healthbarwidget OldValue NewValue true))))

(fn `UserConstructionScript`)