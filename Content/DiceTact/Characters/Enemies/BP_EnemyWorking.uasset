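; BP_EnemyWorking is an enemy character that automatically attacks a nearby hero.
; Each Tick it runs a sphere overlap around itself and casts the results to BP_BaseHeroCharacter.
; The AttackedThisTurn flag limits it to one Attack call; nothing in this graph resets the flag.
; Unconnected nodes hold a debug sphere and a move toward the AI controller's Chariot, neither of which runs.
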(event `self.ReceiveBeginPlay`)

(event `self.ReceiveTick`
  (params (DeltaSeconds :type "Float (single-precision)"))
  (bind _outactors (`KismetSystemLibrary.SphereOverlapActors` (`self.K2_GetActorLocation`) 400.0 (`self.SampledActor`)))
  (for _array_element _outactors
    (bind _asbp_base_hero_character (cast `/Game/DiceTact/Core/BP_BaseHeroCharacter` _array_element))
    (if (not (`self.AttackedThisTurn`))
      (set `self.AttackedThisTurn` true)
      (`self.Attack` _asbp_base_hero_character))))

(fn `UserConstructionScript`)