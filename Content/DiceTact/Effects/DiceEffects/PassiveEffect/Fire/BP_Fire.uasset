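; BP_Fire is a passive dice effect that shows a Niagara fire scaled by the DiceRoll value.
; BeginPlay activates the Fire component, then both it and every Tick map DiceRoll through CurveFireIntensity into User.FireIntensity, printing the result as debug output.
; DoFireIntensity applies the same curve to a passed-in value.
; A random User.FireSpawnRate setter is left disconnected and never runs.
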(event `self.ReceiveBeginPlay`
  (bind _returnvalue (`CurveFloat.GetFloatValue` (`self.CurveFireIntensity`) (`KismetMathLibrary.Conv_IntToDouble` (`self.DiceRoll`))))
  (`ActorComponent.SetActive` (`self.Fire`) true false)
  (`NiagaraComponent.SetVariableFloat` (`self.Fire`) "User.FireIntensity" _returnvalue :!label _label)
  (`KismetSystemLibrary.PrintString` (`KismetStringLibrary.Conv_DoubleToString` _returnvalue)))

(event `Key|One`
  (params (Key :type "Key Structure")))

(event `self.ReceiveTick`
  (params (DeltaSeconds :type "Float (single-precision)"))
  (goto _label))

(fn `DoFireIntensity`
  (params (value :type "Float (double-precision)"))
  (`NiagaraComponent.SetVariableFloat` (`self.Fire`) "User.FireIntensity" (`CurveFloat.GetFloatValue` (`self.CurveFireIntensity`) value)))

(fn `UserConstructionScript`)