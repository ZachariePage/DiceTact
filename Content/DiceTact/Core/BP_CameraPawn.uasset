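; BP_CameraPawn is the player-controlled camera pawn for combat, handling pan, rotation and zoom.
; On possession it adds the combat camera Enhanced Input mapping context.
; Move input is rotated by control yaw and fed to the floating pawn movement, while rotate input adds controller yaw.
; Zoom input sets a clamped target arm length, which Tick interpolates the spring arm toward for smooth zooming.
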(event `self.ReceivePossessed`
  (params (NewController :type "Controller Object Reference"))
  (bind _returnvalue (subsystem `EnhancedInputLocalPlayerSubsystem`))
  (`/Engine/EditorBlueprintResources/StandardMacros.IsValid` _returnvalue
    (:`Is Valid`
      (`EnhancedInputSubsystemInterface.AddMappingContext` _returnvalue "/Game/DiceTact/Core/Input/Combat/IMC_CombatCamera.IMC_CombatCamera" 0 (make `ModifyContextOptions` true false true)))))

(event `EnhancedInput|/Game/DiceTact/Core/Input/Combat/InputActions/IA_Combat_MoveCamera`
  (params (ActionValue :type "Vector2D Structure") (ElapsedSeconds :type "Float (double-precision)") (TriggeredSeconds :type "Float (double-precision)") (InputAction :type "InputAction Object Reference" :default "/Game/DiceTact/Core/Input/Combat/InputActions/IA_Combat_MoveCamera.IA_Combat_MoveCamera"))
  (:`Triggered`
    (`PawnMovementComponent.AddInputVector` (`self.FloatingPawnMovement`) (`KismetMathLibrary.Conv_Vector2DToVector` (`KismetMathLibrary.GetRotated2D` ActionValue (.yaw (`self.GetControlRotation`)))) false)))

(event `self.ReceiveTick`
  (params (DeltaSeconds :type "Float (single-precision)"))
  (bind _springarmcomponent (`self.SpringArmComponent`))
  (set `SpringArmComponent.TargetArmLength` (`KismetMathLibrary.FInterpTo` (`SpringArmComponent.TargetArmLength` _springarmcomponent) (`self.LarpedArmLength`) DeltaSeconds 12.0) _springarmcomponent))

(event `EnhancedInput|/Game/DiceTact/Core/Input/Combat/InputActions/IA_Combat_Zoom`
  (params (ActionValue :type "Float (double-precision)") (ElapsedSeconds :type "Float (double-precision)") (TriggeredSeconds :type "Float (double-precision)") (InputAction :type "InputAction Object Reference" :default "/Game/DiceTact/Core/Input/Combat/InputActions/IA_Combat_Zoom.IA_Combat_Zoom"))
  ;[1 0 0 0.5] Bunch of magic numbers - ALSO FIX AND ACTUALLY USE CAMERA LAG
  (:`Triggered`
    (set `self.LarpedArmLength` (`KismetMathLibrary.FClamp` (+ (`SpringArmComponent.TargetArmLength` (`self.SpringArmComponent`)) (* ActionValue -1.0 (`self.ZoomSpeed`))) (`self.MinArmLength`) (`self.MaxArmLength`)))))

(event `EnhancedInput|/Game/DiceTact/Core/Input/Combat/InputActions/IA_Combat_RotateCam`
  (params (ActionValue :type "Float (double-precision)") (ElapsedSeconds :type "Float (double-precision)") (TriggeredSeconds :type "Float (double-precision)") (InputAction :type "InputAction Object Reference" :default "/Game/DiceTact/Core/Input/Combat/InputActions/IA_Combat_RotateCam.IA_Combat_RotateCam"))
  (:`Triggered`
    (`self.AddControllerYawInput` (* ActionValue (`self.CameraRotationMultiplier`) 1.0))))

(fn `UserConstructionScript`)