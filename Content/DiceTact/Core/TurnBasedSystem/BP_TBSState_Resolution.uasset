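; Turn-based combat state for the Resolution phase, which plays out the pending dice abilities one at a time.
; Each valid die gets camera or combat focus through DTCombatBridgeSubsystem, leaves the PendingAbilities queue and resolves, with its resolve-ended event triggering the next loop step after a short delay.
; Entries with invalid dice are skipped, and an empty queue advances the turn component to the next phase after a pause.
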(event `self.BP_OnStateEntered`
  (`parent.BP_OnStateEntered`)
  (`KismetSystemLibrary.Delay` (`self.OwningTurnBaseComponent`) 0.5)
  (`self.LoopThroughAbilities`))

(event `LoopThroughAbilities`
  (bind _owningturnbasecomponent (`self.OwningTurnBaseComponent`))
  (bind _owningturnbasecomponent_2 (`self.OwningTurnBaseComponent`))
  (bind _pendingabilities (`DTTurnBaseComponent.PendingAbilities` (`self.OwningTurnBaseComponent`)))
  (bind _output (`|GetArrayItem` _pendingabilities))
  (bind ((`DiceActor` _diceactor)) (break `DTPendingAbility` _output))
  (if (`KismetArrayLibrary.Array_IsNotEmpty` _pendingabilities)
    (`/Engine/EditorBlueprintResources/StandardMacros.IsValid` _diceactor
      (:`Is Valid`
        (`DTCombatBridgeSubsystem.RegisterNewFocus` (subsystem `DTCombatBridgeSubsystem` _owningturnbasecomponent_2) _diceactor "Attach")
        (`KismetSystemLibrary.Delay` _owningturnbasecomponent_2 0.3)
        (add `DTDice.OnDiceResolveEnded` _diceactor (`|CreateDelegate` :!event `OnDiceResolved`))
        (bind _output_get (set `self.BindedDice` _diceactor))
        (`KismetArrayLibrary.Array_RemoveItem` (`DTTurnBaseComponent.PendingAbilities` (`self.OwningTurnBaseComponent`)) _output)
        (`DTDice.ResolveDice` _output_get))
      (:`Is Not Valid`
        (`KismetArrayLibrary.Array_RemoveItem` _pendingabilities _output)
        (`self.LoopThroughAbilities`)))
    (else
      (`KismetSystemLibrary.Delay` _owningturnbasecomponent 1.5)
      (`DTTurnBaseComponent.GoToNextPhase` _owningturnbasecomponent))))

(event `OnDiceResolved`
  (remove `DTDice.OnDiceResolveEnded` (`self.BindedDice`) (delegate `OnDiceResolved`))
  (`KismetSystemLibrary.Delay` (`self.OwningTurnBaseComponent`) 0.3)
  (`self.LoopThroughAbilities`))

(event `self.BP_OnStateExit`
  (`parent.BP_OnStateExit`))

(event `self.OnReceiverTurnEnd`)