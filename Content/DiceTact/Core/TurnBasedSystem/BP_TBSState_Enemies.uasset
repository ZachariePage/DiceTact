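; Turn-based system state that runs the enemy phase, giving each opponent turn receiver its turn one at a time.
; On entering, it takes the opponent receivers from the owning turn-base component and shuffles them into a random order.
; It binds and grants authority to the first receiver, removes it from the list, and repeats when that turn ends.
; When the list is empty, it advances the component to the next phase.
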(event `self.BP_OnStateEntered`
  (`parent.BP_OnStateEntered`)
  (bind _output_get (set `self.Opponent Turn Receivers` (`DTTurnBaseComponent.OpponentTurnReceivers` (`self.OwningTurnBaseComponent`))))
  (`KismetArrayLibrary.Array_Shuffle` _output_get)
  (`self.LoopThroughEnemies`))

(event `LoopThroughEnemies`
  (bind _opponent_turn_receivers (`self.Opponent Turn Receivers`))
  (bind _output (`|GetArrayItem` _opponent_turn_receivers))
  (if (`KismetArrayLibrary.Array_IsNotEmpty` _opponent_turn_receivers)
    (`self.BindAndGiveAuthorityTurnReceiver` _output)
    (`KismetArrayLibrary.Array_RemoveItem` _opponent_turn_receivers _output)
    (else
      (`DTTurnBaseComponent.GoToNextPhase` (`self.OwningTurnBaseComponent`)))))

(event `self.OnReceiverTurnEnd`
  (`self.UnbindTurnReceiver`)
  (`self.LoopThroughEnemies`))

(event `self.BP_OnStateExit`)