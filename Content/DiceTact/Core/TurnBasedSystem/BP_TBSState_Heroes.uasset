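; Turn-based system state for the heroes' turn in DiceTact.
; On entry it takes player controller 0 as a DTTurnReceiver, binds to it and hands it the turn.
; When that receiver ends its turn, the state logs a debug message, unbinds it and switches the owning turn-based component to the Resolve state.
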(event `self.BP_OnStateEntered`
  (`parent.BP_OnStateEntered`)
  (bind _asdtturn_receiver (cast `DTTurnReceiver` (`GameplayStatics.GetPlayerController` (`self.OwningTurnBaseComponent`))))
  (`self.BindTurnReceiver` _asdtturn_receiver)
  (`DTTurnReceiver.ReceiveTurn` _asdtturn_receiver))

(event `self.BP_OnStateExit`
  (`parent.BP_OnStateExit`))

(event `self.OnReceiverTurnEnd`
  (bind _owningturnbasecomponent (`self.OwningTurnBaseComponent`))
  (`JUEDevelopmentStatics.ReportDebugMessage` "IT WORKSSS" self (struct :`R` 1.0 :`B` 0.060488 :`A` 1.0))
  (bind _asdtturn_receiver (cast `DTTurnReceiver` (`GameplayStatics.GetPlayerController` _owningturnbasecomponent)))
  (`self.UnbindTurnReceiver` _asdtturn_receiver)
  (`TurnBaseComponent.SetTurnSystemState` _owningturnbasecomponent "/Game/DiceTact/Core/TurnBasedSystem/BP_TBSState_Resolve.BP_TBSState_Resolve_C"))