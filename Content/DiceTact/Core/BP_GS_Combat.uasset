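; Combat GameState that starts and concludes a dice tactics battle.
; BeginPlay late-initializes the elemental reaction and actor factory subsystems, then starts the TurnManager a frame later.
; When combat ends, a win saves cart health and the next level from EncounterBattleInfo, and a modal shows the winner and granted dice.
; Confirmation opens the next level or main menu; a debug event forces the ending, and ResolveEndTurnAbilities only prints.
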(event `self.ReceiveBeginPlay`
  (`ElementalReactionSubsystem.LateInit` (subsystem `ElementalReactionSubsystem`) (`self.Table`))
  (`ActorFactorySubSystem.LateInit` (subsystem `ActorFactorySubSystem`) (`self.Definitions`))
  (`parent.ReceiveBeginPlay`)
  (`KismetSystemLibrary.DelayUntilNextFrame`)
  (`TurnBaseComponent.StartCombat` (`self.TurnManager`)))

(event `self.TurnManager.OnCombatEnded`
  (params (bHeroesWon :type Boolean))
  (bind _heroes_won (`self.Heroes Won`))
  (bind _healthcomponent (`CharetteUnit.HealthComponent` (`TurnBaseComponent.CharetteUnit` (`self.TurnManager`))))
  (set `self.Heroes Won` bHeroesWon)
  (if (`self.Heroes Won`) :!label _label
    (bind _returnvalue (`DTSystemStatics.GetDTGameInstance`))
    (`DiceTactGameInstance.SaveGameCartData` _returnvalue (make `CartGameData` (`HealthComponent.CurrentHealth` _healthcomponent) (`HealthComponent.MaxHealth` _healthcomponent)))
    (bind _returnvalue_2 (`GameplayStatics.GetActorOfClass` "/Script/DiceTact.EncounterBattleInfo"))
    (`DiceTactGameInstance.SetCombatLevel` _returnvalue (select `bool` (`KismetSystemLibrary.IsValid` _returnvalue_2) :`false` "/Game/DiceTact/Maps/Menus/MainMenu.MainMenu" :`true` (`EncounterBattleInfo.NextLevel` _returnvalue_2))))
  (bind _returnvalue_3 (`/JUE/Core/Utilities/BP_JueControllerStatics.PushWidgetToModal` "/Game/DiceTact/UI/Widgets/Combat/WBP_Modal_CombatEnd.WBP_Modal_CombatEnd_C" (`GameplayStatics.GetPlayerController` 0) (`|CreateDelegate` :!event `OnModalConfirmation`)))
  (`/Game/DiceTact/UI/Widgets/Combat/WBP_Modal_CombatEnd.SetWinner` (cast `/Game/DiceTact/UI/Widgets/Combat/WBP_Modal_CombatEnd` _returnvalue_3 :!pure true) _heroes_won (select `bool` _heroes_won :`true` (`EncounterBattleInfo.GrantedDiceOnVictory` _returnvalue_2))))

(event `DEBUG_EndCombat`
  (params (`Heroes Won` :type Boolean))
  (set `self.Heroes Won` `Heroes Won`)
  (goto _label))

(event `OnModalConfirmation`
  (params (Result :type "EModalConfirmationResult Enum" :default "Affirmative"))
  (if (`self.Heroes Won`)
    (`/Game/DiceTact/Utilities/BPFL_SystemStatics.OpenNextLevel`)
    (else
      (`GameplayStatics.OpenLevelBySoftObjectPtr` "/Game/DiceTact/Maps/Menus/MainMenu.MainMenu"))))

(fn `ResolveEndTurnAbilities`
  (`KismetSystemLibrary.PrintString` "gamestate bp"))

(fn `UserConstructionScript`)