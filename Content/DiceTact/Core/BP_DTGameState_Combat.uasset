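; Combat game state for DiceTact that sequences end-of-turn dice resolution.
; On BeginPlay it late-initializes the elemental reaction and actor factory subsystems with table and definition data.
; The resolve event drains the DicesToResolve queue front to back through a latent delay loop, pausing after each die, then calls the next turn.
; ResolveEndTurnAbilities logs a debug string and triggers resolution of pending abilities.
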(event `self.ReceiveBeginPlay`
  (`ElementalReactionSubsystem.LateInit` (subsystem `ElementalReactionSubsystem`) (`self.Table`))
  (`ActorFactorySubSystem.LateInit` (subsystem `ActorFactorySubSystem`) (`self.Definitions`)))

(event `self.OnResolveAbilites`
  (bind _dicestoresolve (`self.DicesToResolve`))
  (if (`KismetArrayLibrary.Array_IsNotEmpty` _dicestoresolve) :!label _label
    (`Dice.ResolveDice` (`|GetArrayItem` _dicestoresolve))
    (`KismetSystemLibrary.Delay` 2.0)
    (`KismetArrayLibrary.Array_Remove` _dicestoresolve)
    (goto _label)
    (else
      (`self.NextTurn`))))

(fn `ResolveEndTurnAbilities`
  (`KismetSystemLibrary.PrintString` "gamestate bp")
  (`self.ResolvePendingAbilities`))

(fn `UserConstructionScript`)