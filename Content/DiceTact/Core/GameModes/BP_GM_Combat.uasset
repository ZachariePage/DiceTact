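; Combat game mode that starts a tactical battle and handles its victory or defeat.
; BeginPlay late-initializes the actor factory subsystem, then starts the TurnManager a frame later.
; When combat ends, or through a debug event, a win stores the cart's health and sets the target level, and a modal announces the winner.
; Confirming the modal saves to disk and opens the overworld on victory, or returns to the main menu on defeat.
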(event `self.ReceiveBeginPlay`
  (`parent.ReceiveBeginPlay`)
  (`DTActorFactorySubSystem.LateInit` (subsystem `DTActorFactorySubSystem`) (`self.Definitions`))
  (`parent.ReceiveBeginPlay`)
  (`KismetSystemLibrary.DelayUntilNextFrame`)
  (`DTTurnBaseComponent.StartCombat` (`self.TurnManager`)))

(event `self.TurnManager.OnCombatEnded`
  (params (bHeroesWon :type Boolean))
  (bind _heroes_won (`self.Heroes Won`))
  (bind _healthcomponent (`DTCharetteUnit.HealthComponent` (`DTTurnBaseComponent.CharetteUnit` (`self.TurnManager`))))
  (set `self.Heroes Won` bHeroesWon)
  (if (`self.Heroes Won`) :!label _label
    (bind _returnvalue (`DTSystemStatics.GetDTGameInstance`))
    (`DiceTactGameInstance.SaveGameCartData` _returnvalue (make `CartGameData` (`DTHealthComponent.CurrentHealth` _healthcomponent) (`DTHealthComponent.MaxHealth` _healthcomponent)))
    (`DiceTactGameInstance.SetTargetLevel` _returnvalue null))
  (bind _returnvalue_2 (`/JUE/Core/Utilities/BP_JueControllerStatics.PushWidgetToModal` "/Game/DiceTact/UI/Widgets/Combat/WBP_Modal_CombatEnd.WBP_Modal_CombatEnd_C" (`GameplayStatics.GetPlayerController` 0) (`|CreateDelegate` :!event `OnModalConfirmation`)))
  (`/Game/DiceTact/UI/Widgets/Combat/WBP_Modal_CombatEnd.SetWinner` (cast `/Game/DiceTact/UI/Widgets/Combat/WBP_Modal_CombatEnd` _returnvalue_2 :!pure true) _heroes_won (select `bool` _heroes_won :!type "DTDiceItemInstance Object Reference")))

(event `DEBUG_EndCombat`
  (params (`Heroes Won` :type Boolean))
  (set `self.Heroes Won` `Heroes Won`)
  (goto _label))

(event `OnModalConfirmation`
  (params (Result :type "EModalConfirmationResult Enum" :default "Affirmative"))
  (if (`self.Heroes Won`)
    (bind _returnvalue (`DTSystemStatics.GetDTGameInstance`))
    (`DiceTactGameInstance.SaveGameToDisk` _returnvalue)
    (`GameplayStatics.OpenLevelBySoftObjectPtr` "/Game/DiceTact/Maps/MainGame/Overworld/Overworld_P.Overworld_P")
    (else
      (`GameplayStatics.OpenLevelBySoftObjectPtr` "/Game/DiceTact/Maps/Menus/MainMenu.MainMenu"))))

(event `self.InitializeHUDForPlayer`
  (params (NewPlayer :type "PlayerController Object Reference"))
  (`WidgetBlueprintLibrary.SetInputMode_GameAndUIEx` NewPlayer null "LockOnCapture" false))

(fn `UserConstructionScript`)