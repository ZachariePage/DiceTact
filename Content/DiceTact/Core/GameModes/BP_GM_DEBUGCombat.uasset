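; Debug combat game mode that starts a battle when play begins and returns to the main menu when it ends.
; BeginPlay late-initializes the actor factory subsystem with Definitions, then waits a frame before the TurnManager starts combat.
; Players get game-and-UI input with the cursor visible during capture.
; When combat ends, a modal shows whether the heroes won, and its confirmation callback opens the MainMenu level.
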(event `self.ReceiveBeginPlay`
  (`parent.ReceiveBeginPlay`)
  (`DTActorFactorySubSystem.LateInit` (subsystem `DTActorFactorySubSystem`) (`self.Definitions`))
  (`KismetSystemLibrary.DelayUntilNextFrame`)
  (`DTTurnBaseComponent.StartCombat` (`self.TurnManager`)))

(event `self.InitializeHUDForPlayer`
  (params (NewPlayer :type "PlayerController Object Reference"))
  (`WidgetBlueprintLibrary.SetInputMode_GameAndUIEx` NewPlayer null "DoNotLock" false))

(event `self.TurnManager.OnCombatEnded`
  (params (bHeroesWon :type Boolean))
  (bind _returnvalue (`/JUE/Core/Utilities/BP_JueControllerStatics.PushWidgetToModal` "/Game/DiceTact/UI/Widgets/Combat/WBP_Modal_CombatEnd.WBP_Modal_CombatEnd_C" (`GameplayStatics.GetPlayerController` 0) (delegate `OnConfimation`)))
  (bind _aswbp_modal_combat_end (cast `/Game/DiceTact/UI/Widgets/Combat/WBP_Modal_CombatEnd` _returnvalue))
  (`/Game/DiceTact/UI/Widgets/Combat/WBP_Modal_CombatEnd.SetWinner` _aswbp_modal_combat_end bHeroesWon null))

(event `OnConfimation`
  (params (Result :type "EModalConfirmationResult Enum" :default "Affirmative"))
  (`GameplayStatics.OpenLevelBySoftObjectPtr` "/Game/DiceTact/Maps/Menus/MainMenu.MainMenu"))

(fn `UserConstructionScript`)