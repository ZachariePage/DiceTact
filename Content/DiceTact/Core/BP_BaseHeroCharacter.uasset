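; Base hero character Blueprint for DiceTact that gives visual feedback when a hero is hovered or selected through interaction events.
; BeginPlay creates dynamic materials for a mesh overlay outline and a selection cylinder.
; Interaction events toggle overlay thickness and recolor both materials for idle, highlighted and committed states, with a Selected flag locking out hover changes.
; Hero tag widget setup and cylinder visibility toggling are present but disconnected.
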(event `self.ReceiveBeginPlay`
  (`parent.ReceiveBeginPlay`)
  (`|ExecutionSequence`
    (:`then_0`
      (`/Engine/EditorBlueprintResources/StandardMacros.Create and Assign MID` (`self.OverlayMID`) "/Game/DiceTact/MaterialLibrary/M_Overlay.M_Overlay"
        (:`Out`
          (`MeshComponent.SetOverlayMaterial` (`self.Mesh`) (`self.OverlayMID`))
          (`/Engine/EditorBlueprintResources/StandardMacros.Create and Assign MID` (`self.CylinderMID`) (`PrimitiveComponent.GetMaterial` (`self.SelectionCylinder`) 0)
            (:`Out`
              (`PrimitiveComponent.SetMaterial` (`self.SelectionCylinder`) 0 (`self.CylinderMID`))
              (`self.SetSelectionActive` false)
              (`self.UpdateOverlayColor` (struct :`R` 1.0 :`G` 1.0 :`B` 1.0 :`A` 1.0)))))))))

(event `self.BeginInteraction`
  (params (InteractionQuery :type "InteractionQuery Structure (by ref)"))
  (if (not (`self.bSelected`))
    (`self.SetSelectionActive` true)
    (`self.UpdateOverlayColor` (struct :`R` 0.095216 :`G` 1.0 :`A` 1.0))))

(event `self.StopInteraction`
  (params (InteractionQuery :type "InteractionQuery Structure (by ref)"))
  (if (not (`self.bSelected`))
    (`self.SetSelectionActive` false)
    (`self.UpdateOverlayColor` (struct :`R` 1.0 :`G` 1.0 :`B` 1.0 :`A` 1.0))))

(event `self.TryCommitInteraction`
  (params (InteractionQuery :type "InteractionQuery Structure (by ref)"))
  (set `self.bSelected` true)
  (`self.SetSelectionActive` true)
  (`self.UpdateOverlayColor` (struct :`R` 1.0 :`B` 0.32491 :`A` 1.0)))

(event `self.CancelInteractionCommit`
  (params (InteractionQuery :type "InteractionQuery Structure (by ref)"))
  (set `self.bSelected` false)
  (`self.SetSelectionActive` false)
  (`self.UpdateOverlayColor` (struct :`R` 1.0 :`G` 1.0 :`B` 1.0 :`A` 1.0)))

(fn `SetSelectionActive`
  (params (bActive :type Boolean))
  (`MaterialInstanceDynamic.SetScalarParameterValue` (`self.OverlayMID`) "BaseThickness" (`KismetMathLibrary.SelectFloat` 1.0 0.0 bActive)))

(fn `UpdateOverlayColor`
  (params (NewColor :type "LinearColor Structure"))
  (`MaterialInstanceDynamic.SetVectorParameterValue` (`self.OverlayMID`) "Color" NewColor)
  (`MaterialInstanceDynamic.SetVectorParameterValue` (`self.CylinderMID`) "Color" NewColor))

(fn `UserConstructionScript`)