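; Debug combat game state for the DiceTact dice game that sets up actor creation and resolves queued dice.
; On BeginPlay it passes its Definitions to the actor factory subsystem for late initialization.
; OnResolveAbilites works through DicesToResolve sequentially in a delayed loop, resolving the first die, pausing, then removing it until the queue is empty.
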(event `self.ReceiveBeginPlay`
  (`ActorFactorySubSystem.LateInit` (subsystem `ActorFactorySubSystem`) (`self.Definitions`)))

(event `self.OnResolveAbilites`
  (bind _dicestoresolve (`self.DicesToResolve`))
  (if (`KismetArrayLibrary.Array_IsNotEmpty` _dicestoresolve) :!label _label
    (`Dice.ResolveDice` (`|GetArrayItem` _dicestoresolve))
    (`KismetSystemLibrary.Delay` 5.0)
    (`KismetArrayLibrary.Array_Remove` _dicestoresolve)
    (goto _label)))

(fn `UserConstructionScript`)