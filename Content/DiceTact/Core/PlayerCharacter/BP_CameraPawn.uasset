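; Player-controlled combat camera pawn that moves, rotates and zooms, and can focus on actors.
; Enhanced Input drives yaw-relative panning through FloatingPawnMovement, controller yaw rotation, and a clamped spring-arm length target that Tick interpolates toward.
; DTCombatBridgeSubsystem focus events either snap the camera once, set an actor for Tick to follow until unfocused, or center it on a group's average location.
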(event `self.ReceivePossessed`
  (params (NewController :type "Controller Object Reference"))
  (bind _returnvalue (subsystem `EnhancedInputLocalPlayerSubsystem`))
  (`/Engine/EditorBlueprintResources/StandardMacros.IsValid` _returnvalue
    (:`Is Valid`
      (`EnhancedInputSubsystemInterface.AddMappingContext` _returnvalue "/Game/DiceTact/Core/Input/Combat/IMC_CombatCamera.IMC_CombatCamera" 0 (make `ModifyContextOptions` true false true)))))

(event `self.ReceiveBeginPlay`
  (bind _returnvalue (subsystem `DTCombatBridgeSubsystem`))
  (`parent.ReceiveBeginPlay`)
  (`/Engine/EditorBlueprintResources/StandardMacros.IsValid` _returnvalue
    (:`Is Valid`
      (add `DTCombatBridgeSubsystem.OnNewActorFocus` _returnvalue (delegate `OnNewAuthority`))
      (add `DTCombatBridgeSubsystem.OnActorsFocused` _returnvalue (`|CreateDelegate` :!event `OnActorsFocused`)))))

(event `OnNewAuthority`
  (params (FocusedActor :type "Actor Object Reference") (FocusMethod :type "EFocusActorMethod Enum" :default "SnapOnce") (bIsFocused :type Boolean))
  (if bIsFocused
    (`/Engine/EditorBlueprintResources/StandardMacros.IsValid` FocusedActor
      (:`Is Valid`
        (if (`|EnumEquality` FocusMethod "SnapOnce")
          (`self.SetNewLocation` (`self.K2_GetActorLocation` FocusedActor))
          (else
            (set `self.Focused Actor` FocusedActor)))))
    (elif (`KismetSystemLibrary.IsValid` (`self.Focused Actor`))
      (set `self.Focused Actor` null))))

(event `OnActorsFocused`
  (params (FocusedActors :type "Array of Actor Object Reference (by ref)"))
  (bind _returnvalue (`GameplayStatics.GetActorArrayAverageLocation` FocusedActors))
  (`self.SetNewLocation` _returnvalue))

(event `EnhancedInput|/Game/DiceTact/Core/Input/Combat/InputActions/IA_Combat_MoveCamera`
  (params (ActionValue :type "Vector2D Structure") (ElapsedSeconds :type "Float (double-precision)") (TriggeredSeconds :type "Float (double-precision)") (InputAction :type "InputAction Object Reference" :default "/Game/DiceTact/Core/Input/Combat/InputActions/IA_Combat_MoveCamera.IA_Combat_MoveCamera"))
  (:`Triggered`
    (`PawnMovementComponent.AddInputVector` (`self.FloatingPawnMovement`) (`KismetMathLibrary.Conv_Vector2DToVector` (`KismetMathLibrary.GetRotated2D` ActionValue (.yaw (`self.GetControlRotation`)))) false)))

(event `self.ReceiveTick`
  (params (DeltaSeconds :type "Float (single-precision)"))
  (bind _focused_actor (`self.Focused Actor`))
  (bind _springarmcomponent (`self.SpringArmComponent`))
  (set `SpringArmComponent.TargetArmLength` (`KismetMathLibrary.FInterpTo` (`SpringArmComponent.TargetArmLength` _springarmcomponent) (`self.LarpedArmLength`) (* (`GameplayStatics.GetGlobalTimeDilation`) DeltaSeconds) 12.0) _springarmcomponent)
  (`/Engine/EditorBlueprintResources/StandardMacros.IsValid` _focused_actor
    (:`Is Valid`
      (`SceneComponent.K2_SetWorldLocation` (`self.RootSceneComponent`) (`self.K2_GetActorLocation` _focused_actor) false false))))

(event `EnhancedInput|/Game/DiceTact/Core/Input/Combat/InputActions/IA_Combat_Zoom`
  (params (ActionValue :type "Float (double-precision)") (ElapsedSeconds :type "Float (double-precision)") (TriggeredSeconds :type "Float (double-precision)") (InputAction :type "InputAction Object Reference" :default "/Game/DiceTact/Core/Input/Combat/InputActions/IA_Combat_Zoom.IA_Combat_Zoom"))
  ;[1 0 0 0.5] Bunch of magic numbers - ALSO FIX AND ACTUALLY USE CAMERA LAG
  (:`Triggered`
    (set `self.LarpedArmLength` (`KismetMathLibrary.FClamp` (+ (`SpringArmComponent.TargetArmLength` (`self.SpringArmComponent`)) (* ActionValue -1.0 (`self.ZoomSpeed`))) (`self.DefaultMinArmLength`) (`self.DefaultMaxArmLength`)))))

(event `EnhancedInput|/Game/DiceTact/Core/Input/Combat/InputActions/IA_Combat_RotateCam`
  (params (ActionValue :type "Float (double-precision)") (ElapsedSeconds :type "Float (double-precision)") (TriggeredSeconds :type "Float (double-precision)") (InputAction :type "InputAction Object Reference" :default "/Game/DiceTact/Core/Input/Combat/InputActions/IA_Combat_RotateCam.IA_Combat_RotateCam"))
  (:`Triggered`
    (`self.AddControllerYawInput` (* ActionValue (`self.CameraRotationMultiplier`) 1.0))))

(fn `SetNewLocation`
  (params (NewLocation :type "Vector Structure"))
  (`SceneComponent.K2_SetRelativeLocation` (`self.RootSceneComponent`) NewLocation false false))

(fn `UserConstructionScript`)