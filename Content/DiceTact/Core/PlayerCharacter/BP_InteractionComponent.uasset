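; Player controller component that drives cursor-based interaction with actors implementing an interaction interface.
; Each tick it traces under the cursor, tracks the hovered actor and sends begin and stop messages as the target changes.
; Commit and cancel events forward to that actor, and event dispatchers broadcast both hover and commit changes.
; Every message carries a query naming the controller as instigator, and disabling interaction releases the current target.
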(event `self.ReceiveBeginPlay`
  (`parent.ReceiveBeginPlay`)
  (bind _asplayer_controller (cast `PlayerController` (`self.GetOwner`)))
  (set `self.PlayerController` _asplayer_controller))

(event `self.ReceiveTick`
  (params (DeltaSeconds :type "Float (single-precision)"))
  (bind _playercontroller (`self.PlayerController`))
  (bind _interactableactor (`self.InteractableActor`))
  (bind _interactableactor_2 (`self.InteractableActor`))
  (bind _playercontroller_2 (`self.PlayerController`))
  (bind _interactionquery (make `InteractionQuery` _playercontroller _playercontroller))
  (bind (_bblockinghit _binitialoverlap _time _distance _location _impactpoint _normal _impactnormal _physmat _hitactor) (`GameplayStatics.BreakHitResult` (`PlayerController.GetHitResultUnderCursorByChannel` (`self.PlayerController`) "TraceTypeQuery4" true)))
  (if (and (`self.InteractionEnabled`) _bblockinghit (`KismetSystemLibrary.DoesImplementInterface` _hitactor))
    (if (not (== _hitactor (`self.InteractableActor`)))
      (`/Engine/EditorBlueprintResources/StandardMacros.IsValid` _interactableactor_2
        (:`Is Valid`
          (message `DTInteractable.StopInteraction` _interactableactor_2 _interactionquery)
          (`self.OnPreInteraction` false _interactableactor_2))
        (:`Is Not Valid`
          _))
      (bind _output_get (set `self.InteractableActor` _hitactor))
      (`self.BeginInteraction` _output_get _interactionquery))
    (else
      (`/Engine/EditorBlueprintResources/StandardMacros.IsValid` _interactableactor
        (:`Is Valid`
          (message `DTInteractable.StopInteraction` _interactableactor (make `InteractionQuery` _playercontroller_2 _playercontroller_2))
          (set `self.InteractableActor` null)
          (`self.OnPreInteraction` false))))))

(event `CommitInteraction`
  (bind _playercontroller (`self.PlayerController`))
  (bind _interactableactor (`self.InteractableActor`))
  (`/Engine/EditorBlueprintResources/StandardMacros.IsValid` _interactableactor
    (:`Is Valid`
      (message `DTInteractable.TryCommitInteraction` _interactableactor (make `InteractionQuery` _playercontroller _playercontroller))
      (`self.OnCommitInteraction` true))))

(event `CancelInteraction`
  (bind _interactableactor (`self.InteractableActor`))
  (bind _playercontroller (`self.PlayerController`))
  (`/Engine/EditorBlueprintResources/StandardMacros.IsValid` _interactableactor
    (:`Is Valid`
      (message `DTInteractable.CancelInteractionCommit` _interactableactor (make `InteractionQuery` _playercontroller _playercontroller))
      (`self.OnCommitInteraction` false))))

(event `SetInteractionEnabled`
  (params (bEnabled :type Boolean))
  (bind _interactableactor (`self.InteractableActor`))
  (bind _playercontroller (`self.PlayerController`))
  (bind _output_get (set `self.InteractionEnabled` bEnabled))
  (if (not _output_get)
    (`/Engine/EditorBlueprintResources/StandardMacros.IsValid` _interactableactor
      (:`Is Valid`
        (message `DTInteractable.StopInteraction` _interactableactor (make `InteractionQuery` _playercontroller _playercontroller))
        (`self.OnPreInteraction` false _interactableactor)
        (set `self.InteractableActor` null)))))

(fn `BeginInteraction`
  (params (InteractedActor :type "Actor Object Reference") (InteractionQuery :type "InteractionQuery Structure (by ref)"))
  (message `DTInteractable.BeginInteraction` InteractedActor InteractionQuery)
  (`self.OnPreInteraction` true InteractedActor))