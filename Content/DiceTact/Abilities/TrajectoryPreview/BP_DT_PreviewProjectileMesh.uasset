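; Trajectory preview actor that draws a projectile path as spline meshes, with a marker shown only for valid placement.
; UpdateSplinePoints rebuilds the spline, then adds or destroys segment components to follow the point count.
; UpdateCurrentMesh refits segments to the spline and applies an overlay material when the count matches or shrinks, but not when it grows.
; UpdateEndMesh only toggles marker visibility, ignoring the hit result, and UpdateCurrentMeshes is not called here.
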(event `self.ReceiveBeginPlay`
  (`parent.ReceiveBeginPlay`)
  (`SceneComponent.SetVisibility` (`self.ValidPlacementPreview`) false false))

(event `UpdateSplinePoints`
  (params (Points :type "Array of Vector Structure") (CoordinateSpace :type "ESplineCoordinateSpace Enum" :default "Local"))
  (bind _returnvalue (`KismetArrayLibrary.Array_Length` Points))
  (bind _splinemeshes (`self.SplineMeshes`))
  (bind _splinemeshes_2 (`self.SplineMeshes`))
  (bind _spline (`self.Spline`))
  (bind _returnvalue_2 (`KismetArrayLibrary.Array_Length` (`self.SplineMeshes`)))
  (bind _output (`|GetArrayItem` _splinemeshes_2 (`KismetArrayLibrary.Array_LastIndex` _splinemeshes_2)))
  (`SplineComponent.SetSplinePoints` (`self.Spline`) Points CoordinateSpace true)
  (`/Engine/EditorBlueprintResources/StandardMacros.CompareInt` _returnvalue _returnvalue_2
    (:`>`
      (for _index (range (- _returnvalue _returnvalue_2))
        (`SplineComponent.SetSplinePointType` (`self.Spline`) _index "CurveClamped" true)
        (bind _returnvalue_3 (`AddComponent|NODE_AddSplineMeshComponent-2` :`bManualAttachment` true))
        (`KismetArrayLibrary.Array_Add` (`self.SplineMeshes`) _returnvalue_3)
        (bind _returnvalue_4 (+ _index _returnvalue_2))
        (bind (_location _tangent) (`SplineComponent.GetLocationAndTangentAtSplinePoint` _spline _returnvalue_4 "Local"))
        (bind (_location_2 _tangent_2) (`SplineComponent.GetLocationAndTangentAtSplinePoint` _spline (+ _returnvalue_4 1) "Local"))
        (`SplineMeshComponent.SetStartAndEnd` _returnvalue_3 _location _tangent _location_2 _tangent_2 true)
        (`SceneComponent.K2_AttachToComponent` _returnvalue_3 (`self.DefaultSceneRoot`) "None" "KeepRelative" "KeepRelative" "KeepRelative" true)))
    (:`==`
      (`self.UpdateCurrentMesh`))
    (:`<`
      (for _ (range (+ (- _returnvalue_2 _returnvalue) 1))
        (if (and (`KismetSystemLibrary.IsValid` _output) (not (`ActorComponent.IsBeingDestroyed` _output)))
          (`ActorComponent.K2_DestroyComponent` _output)
          (`KismetArrayLibrary.Array_Remove` _splinemeshes (`KismetArrayLibrary.Array_LastIndex` _splinemeshes))))
      (`self.UpdateCurrentMesh`))))

(event `UpdateEndMesh`
  (params (HitResult :type "HitResult Structure (by ref)") (ValidPlacement :type Boolean))
  (`SceneComponent.SetVisibility` (`self.ValidPlacementPreview`) ValidPlacement false))

(fn `UpdateCurrentMesh`
  (bind _spline (`self.Spline`))
  (for _index (range (+ (- (`SplineComponent.GetNumberOfSplinePoints` (`self.Spline`)) 0) 1))
    (bind _output (`|GetArrayItem` (`self.SplineMeshes`) _index))
    (`/Engine/EditorBlueprintResources/StandardMacros.IsValid` _output
      (:`Is Valid`
        (bind (_location _tangent) (`SplineComponent.GetLocationAndTangentAtSplinePoint` _spline _index "Local"))
        (bind (_location_2 _tangent_2) (`SplineComponent.GetLocationAndTangentAtSplinePoint` _spline (+ _index 1) "Local"))
        (`SplineMeshComponent.SetStartAndEnd` _output _location _tangent _location_2 _tangent_2 true)
        (`PrimitiveComponent.SetMaterial` _output 0 "/Game/DiceTact/MaterialLibrary/M_Overlay.M_Overlay")))))

(fn `UpdateCurrentMeshes`
  (params (InputPin :type "Array of Vector Structure"))
  (bind _splinemeshes (`self.SplineMeshes`))
  (if (`KismetArrayLibrary.Array_IsNotEmpty` _splinemeshes)
    (for _index (range (`KismetArrayLibrary.Array_Length` _splinemeshes))
      (bind _returnvalue (+ _index 1))
      (if (== _returnvalue (`KismetArrayLibrary.Array_Length` InputPin))
        (break)
        (else
          (bind _output (`|GetArrayItem` _splinemeshes _index))
          (bind _output_2 (`|GetArrayItem` InputPin _index))
          (`SceneComponent.K2_SetRelativeLocation` _output _output_2 false false)
          (`SplineMeshComponent.SetStartAndEnd` _output (0.0 0.0 0.0) (0.0 0.0 0.0) (- (`|GetArrayItem` InputPin _returnvalue) _output_2) (0.0 0.0 0.0) true))))
    (return)))

(fn `UserConstructionScript`)