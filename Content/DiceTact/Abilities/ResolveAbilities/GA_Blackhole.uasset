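; GA_Blackhole is a resolve gameplay ability that spawns a short-lived BP_Collapser at the owner actor's location.
; On activation it commits, then draws a debug sphere whose radius scales with ability level from its Data values.
; That radius is not passed to the collapser, which is destroyed after a brief delay.
; The graph never calls EndAbility.
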(event `self.K2_ActivateAbility`
  (bind _returnvalue (`Actor.K2_GetActorLocation` (`.OwnerActor` (break `GameplayAbilityActorInfo` (`self.GetActorInfo`)))))
  (`self.K2_CommitAbility`)
  (`KismetSystemLibrary.DrawDebugSphere` _returnvalue (+ (`DTBlackHoleData.BaseRadius` (`self.data`)) (* (`DTBlackHoleData.AdditionalRadius` (`self.data`)) (`self.GetAbilityLevel`))) 12 (struct :`R` 1.0 :`G` 1.0 :`B` 1.0 :`A` 1.0) 3.0 1.0)
  (bind _returnvalue_2 (`|SpawnActorFromClass` "/Game/Vefects/Vertex_Collapse_VFX/VFX/BP/BP_Collapser.BP_Collapser_C" (`KismetMathLibrary.Conv_VectorToTransform` _returnvalue) "Undefined" "MultiplyWithRoot" null (0.0 0.0 0.0) (struct :`R` 1.0 :`G` 0.059511 :`A` 1.0) (0.1 0.5 0.0) 100.0 0.5 100.0 1.0 0.0 true 1.0 1.0 null))
  (`KismetSystemLibrary.Delay` 1.0)
  (`Actor.K2_DestroyActor` _returnvalue_2))