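; BP_MovePreview is the movement preview in DiceTact, showing whether a move is valid by the color of its mesh.
; On BeginPlay it creates a dynamic material instance from PreviewMesh's first material and assigns it back to that slot.
; SetValidMovement then sets that instance's Color parameter to green for a valid move or red for an invalid one.
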(event `self.ReceiveBeginPlay`
  (`parent.ReceiveBeginPlay`)
  (`/Engine/EditorBlueprintResources/StandardMacros.Create and Assign MID` (`self.MID`) (`PrimitiveComponent.GetMaterial` (`self.PreviewMesh`) 0)
    (:`Out`
      (`PrimitiveComponent.SetMaterial` (`self.PreviewMesh`) 0 (`self.MID`)))))

(event `SetValidMovement`
  (params (bValidMove :type Boolean))
  (`MaterialInstanceDynamic.SetVectorParameterValue` (`self.MID`) "Color" (select `bool` bValidMove :`false` (struct :`R` 1.0 :`A` 1.0) :`true` (struct :`G` 1.0 :`B` 0.058355 :`A` 1.0) :!type "LinearColor Structure")))

(fn `UserConstructionScript`)