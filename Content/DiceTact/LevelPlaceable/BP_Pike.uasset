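; BP_Pike is a level-placeable spike hazard that damages and knocks back whatever hits it.
; On Hit, any Damageable not on cooldown takes 1 damage, and an EnemyUnit is also pushed away from the pike via PushTowardBlackHole.
; The EnemieHit map stores a one-second cooldown per hit actor, which Tick counts down and removes on expiry.
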(event `self.ReceiveTick`
  (params (DeltaSeconds :type "Float (single-precision)"))
  (bind (_keypin _valuepin) (`|MapForEach` (`self.EnemieHit`))
    (:`then`
      (bind _returnvalue (- _valuepin DeltaSeconds))
      (`BlueprintMapLibrary.Map_Add` (`self.EnemieHit`) _keypin _returnvalue)
      (if (< _returnvalue 0.0)
        (`BlueprintMapLibrary.Map_Remove` (`self.EnemieHit`) _keypin)))))

(event `self.ReceiveHit`
  (params (MyComp :type "PrimitiveComponent Object Reference") (Other :type "Actor Object Reference") (OtherComp :type "PrimitiveComponent Object Reference") (bSelfMoved :type Boolean) (HitLocation :type "Vector Structure") (HitNormal :type "Vector Structure") (NormalImpulse :type "Vector Structure") (Hit :type "HitResult Structure (by ref)"))
  (if (not (`BlueprintMapLibrary.Map_Contains` (`self.EnemieHit`) Other))
    (bind _asdamageable (cast `Damageable` Other))
    (`Damageable.TakeDamage` _asdamageable self 1)
    (`BlueprintMapLibrary.Map_Add` (`self.EnemieHit`) Other 1.0)
    (bind _asenemy_unit (cast `EnemyUnit` Other))
    (`Pushable.PushTowardBlackHole` _asenemy_unit (make `PushData` (`KismetMathLibrary.GetDirectionUnitVector` (`self.K2_GetActorLocation` self) (`self.K2_GetActorLocation` Other)) 800.0 self))
    (`KismetSystemLibrary.PrintString` "Hello")))

(fn `UserConstructionScript`)