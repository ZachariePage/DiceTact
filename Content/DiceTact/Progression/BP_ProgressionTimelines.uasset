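; BP_ProgressionTimelines is an actor that provides a timed 2D move-to-location animation for the progression system.
; On BeginPlay it sets the MoveToLocation timeline's play rate from AnimCompletionTime.
; StartMoveToLocationAnimation stores Start and End, then plays the timeline, broadcasting the interpolated position on each update and a separate event on finish.
; Interpolation converts the Vector2D values to 3D vectors for Lerp, then back.
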(event `self.ReceiveBeginPlay`
  (`parent.ReceiveBeginPlay`)
  (`TimelineComponent.SetPlayRate` (`self.MoveToLocation`) (/ 1.0 (`self.AnimCompletionTime`))))

(event `StartMoveToLocationAnimation`
  (params (Start :type "Vector2D Structure") (End :type "Vector2D Structure"))
  (bind _output_get (set `self.Start` Start))
  (bind _output_get_2 (set `self.End` End))
  (bind (_direction _alpha) (`Timeline|MoveToLocation` :!via `PlayFromStart`)
    (:`Update`
      (`self.OnMoveToLocAnimUpdate` (`KismetMathLibrary.Conv_VectorToVector2D` (`KismetMathLibrary.VLerp` (`KismetMathLibrary.Conv_Vector2DToVector` _output_get) (`KismetMathLibrary.Conv_Vector2DToVector` _output_get_2) _alpha))))
    (:`Finished`
      (`self.OnMoveToLocAnimFinished`))))

(fn `UserConstructionScript`)