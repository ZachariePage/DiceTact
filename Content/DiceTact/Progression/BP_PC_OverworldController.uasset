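; Player controller for the overworld map screen, handling its UI setup and input.
; On BeginPlay it adds the navigation and menu input contexts, pushes the overworld map widget to the game layer and initializes it with the progression timelines actor from its child actor component.
; The camera-move action navigates the map, and the open-menu action pushes the pause menu widget to the menu layer.
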(event `self.ReceiveBeginPlay`
  (bind _returnvalue (pcsubsystem `EnhancedInputLocalPlayerSubsystem` self))
  (`parent.ReceiveBeginPlay`)
  (`EnhancedInputSubsystemInterface.AddMappingContext` _returnvalue "/Game/DiceTact/Core/Input/IMC_Overworld_Navigation.IMC_Overworld_Navigation" 0 (make `ModifyContextOptions` true false true))
  (`EnhancedInputSubsystemInterface.AddMappingContext` _returnvalue "/Game/DiceTact/Core/Input/Menu/IMC_Menu.IMC_Menu" 0 (make `ModifyContextOptions` true false true))
  (bind _pushedwidget (`/JUE/Core/Utilities/BP_JueControllerStatics.PushWidgetToGame` "/Game/DiceTact/Progression/Widgets/WBP_OverworldMap.WBP_OverworldMap_C" self))
  (bind _output_get (set `self.OverworldMap` (cast `/Game/DiceTact/Progression/Widgets/WBP_OverworldMap` _pushedwidget :!pure true)))
  (bind _asbp_progression_timelines (cast `/Game/DiceTact/Progression/BP_ProgressionTimelines` (`ChildActorComponent.ChildActor` (`self.ChildActor`))))
  (`/Game/DiceTact/Progression/Widgets/WBP_OverworldMap.InitializeOverworld` _output_get _asbp_progression_timelines))

(event `EnhancedInput|/Game/DiceTact/Core/Input/Combat/InputActions/IA_Combat_MoveCamera`
  (params (ActionValue :type "Vector2D Structure") (ElapsedSeconds :type "Float (double-precision)") (TriggeredSeconds :type "Float (double-precision)") (InputAction :type "InputAction Object Reference" :default "/Game/DiceTact/Core/Input/Combat/InputActions/IA_Combat_MoveCamera.IA_Combat_MoveCamera"))
  (:`Triggered`
    (`/Game/DiceTact/Progression/Widgets/WBP_OverworldMap.NavigateMap` (`self.OverworldMap`) ActionValue)))

(event `EnhancedInput|/Game/DiceTact/Core/Input/Menu/InputActions/IA_OpenMenu`
  (params (ActionValue :type Boolean) (ElapsedSeconds :type "Float (double-precision)") (TriggeredSeconds :type "Float (double-precision)") (InputAction :type "InputAction Object Reference" :default "/Game/DiceTact/Core/Input/Menu/InputActions/IA_OpenMenu.IA_OpenMenu"))
  (:`Triggered`
    (`/JUE/Core/Utilities/BP_JueControllerStatics.PushWidgetToMenu` "/Game/DiceTact/UI/Widgets/Menus/WBP_Overworld_PauseMenu.WBP_Overworld_PauseMenu_C" self)))

(fn `UserConstructionScript`)