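; BP_OL_Workshop is the Workshop travel location, offering the player an upgrade to the cart's max health.
; On player travel it pushes WBP_WorkshopWidget to a modal, passes in the amount from GetCartMaxHealthUpgrade and refreshes its text.
; The confirmation callback has the widget apply the health increase, then finishes travel, without checking the result value.
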(event `self.OnPlayerTravel`
  (bind _returnvalue (`Widget.GetOwningPlayer` (`self.OwnerLocationWidget`)))
  (bind _returnvalue_2 (`/JUE/Core/Utilities/BP_JueControllerStatics.PushWidgetToModal` "/Game/DiceTact/Progression/Widgets/WBP_WorkshopWidget.WBP_WorkshopWidget_C" _returnvalue (delegate `OnConfirmation`) _returnvalue))
  (bind _aswbp_workshop_widget (cast `/Game/DiceTact/Progression/Widgets/WBP_WorkshopWidget` _returnvalue_2))
  (bind _output_get (set `self.As WBP Workshop Widget` _aswbp_workshop_widget))
  (set `/Game/DiceTact/Progression/Widgets/WBP_WorkshopWidget.MaxHealthAdded` (`self.GetCartMaxHealthUpgrade`) _output_get)
  (`/Game/DiceTact/Progression/Widgets/WBP_WorkshopWidget.UpdateText` (`self.As WBP Workshop Widget`)))

(event `OnConfirmation`
  (params (Result :type "EModalConfirmationResult Enum" :default "Affirmative"))
  (`/Game/DiceTact/Progression/Widgets/WBP_WorkshopWidget.AddCartMaxHealth` (`self.As WBP Workshop Widget`))
  (`self.FinishTravel`))