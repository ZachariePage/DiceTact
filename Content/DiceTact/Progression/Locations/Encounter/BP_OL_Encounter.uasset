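; Encounter location logic that takes the player from a location widget into that location's encounter map.
; On player travel it validates the map reference, sets it as the game instance's target level and sets the location identifier as current in the loaded save.
; It then pushes a fade widget and opens the next level once the fade animation ends, or reports an error if no map is set.
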(event `self.OnPlayerTravel`
  (bind _ownerlocationwidget (`self.OwnerLocationWidget`))
  (if (`KismetSystemLibrary.IsValidSoftObjectReference` (`self.EncounterMap`))
    (bind _returnvalue (`DTSystemStatics.GetDTGameInstance`))
    (`DiceTactGameInstance.SetTargetLevel` _returnvalue (`self.EncounterMap`))
    (`DiceTactSaveGame.SetCurrentLocation` (`DiceTactGameInstance.GetLoadedGameSave` _returnvalue) (`DTOverworldLocationWidget.LocationIdentifier` _ownerlocationwidget))
    (bind _returnvalue_2 (`/JUE/Core/Utilities/BP_JueControllerStatics.PushWidgetToMenu` "/JUE/UI/WBP_Fade.WBP_Fade_C" (`Widget.GetOwningPlayer` _ownerlocationwidget) _ownerlocationwidget))
    (bind _output_get (set `self.WBP Fade` (cast `/JUE/UI/WBP_Fade` _returnvalue_2 :!pure true)))
    (set `/JUE/UI/WBP_Fade.bFadeOutAutomatically` false _output_get)
    (set `/JUE/UI/WBP_Fade.FadeAnimTime` 0.4 _output_get)
    (add `/JUE/UI/WBP_Fade.OnFadeAnimEnd` _output_get (`|CreateDelegate` :!event `OnFadeEnd`))
    (`/JUE/UI/WBP_Fade.StartFadeAnimation` _output_get)
    (else
      (`JUEDevelopmentStatics.ReportErrorMessage` "Could not Save encounter map, because it is not set!" self))))

(event `OnFadeEnd`
  (params (PlayMode :type "EUMGSequencePlayMode Enum" :default "Forward"))
  (`/Game/DiceTact/Utilities/BPFL_SystemStatics.OpenNextLevel` (`self.OwnerLocationWidget`)))