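; Collapser actor that drives a vertex collapse effect by writing its settings to a shared Material Parameter Collection.
; Every tick it pushes its offset position, axis, color, emissive intensity, hardness, sine frequency and collapse intensity.
; A timeline started at BeginPlay animates the collapse radius between base and multiplied values, also scaling a debug sphere.
; The construction script offsets that sphere and toggles its visibility with a debug flag.
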(event `self.ReceiveTick`
  (params (DeltaSeconds :type "Float (single-precision)"))
  (`|ExecutionSequence`
    (:`then_0`
      (`KismetMaterialLibrary.SetVectorParameterValue` "/Game/Vefects/Vertex_Collapse_VFX/VFX/Materials/Collections/MPC_Vefects_Vertex_Collapse_01.MPC_Vefects_Vertex_Collapse_01" "CollapsePos" (`KismetMathLibrary.Conv_VectorToLinearColor` (+ (`self.K2_GetActorLocation`) (`self.PosOffset`))))
      (`KismetMaterialLibrary.SetVectorParameterValue` "/Game/Vefects/Vertex_Collapse_VFX/VFX/Materials/Collections/MPC_Vefects_Vertex_Collapse_01.MPC_Vefects_Vertex_Collapse_01" "CollapseEmColor" (`self.Color`))
      (`KismetMaterialLibrary.SetVectorParameterValue` "/Game/Vefects/Vertex_Collapse_VFX/VFX/Materials/Collections/MPC_Vefects_Vertex_Collapse_01.MPC_Vefects_Vertex_Collapse_01" "CollapseAxis" (`KismetMathLibrary.Conv_VectorToLinearColor` (`self.Axis`))))
    (:`then_1`
      (`KismetMaterialLibrary.SetScalarParameterValue` "/Game/Vefects/Vertex_Collapse_VFX/VFX/Materials/Collections/MPC_Vefects_Vertex_Collapse_01.MPC_Vefects_Vertex_Collapse_01" "CollapseEmIntensity" (`self.EmIntensity`))
      (`KismetMaterialLibrary.SetScalarParameterValue` "/Game/Vefects/Vertex_Collapse_VFX/VFX/Materials/Collections/MPC_Vefects_Vertex_Collapse_01.MPC_Vefects_Vertex_Collapse_01" "CollapseHardness" (`self.Hardness`))
      (`KismetMaterialLibrary.SetScalarParameterValue` "/Game/Vefects/Vertex_Collapse_VFX/VFX/Materials/Collections/MPC_Vefects_Vertex_Collapse_01.MPC_Vefects_Vertex_Collapse_01" "CollapseSineFrequency" (`self.SineFreq`))
      (`KismetMaterialLibrary.SetScalarParameterValue` "/Game/Vefects/Vertex_Collapse_VFX/VFX/Materials/Collections/MPC_Vefects_Vertex_Collapse_01.MPC_Vefects_Vertex_Collapse_01" "CollapseIntensity" (`self.CollapseIntensity`)))
    (:`then_2`
      (`TimelineComponent.SetPlayRate` (`self.RadiusDemo`) (`self.DebugSpeed`)))))

(event `self.ReceiveBeginPlay`
  (bind _radius (`self.Radius`))
  (bind (_direction _newtrack_0) (`Timeline|RadiusDemo` :`NewTime` (`self.DebugSpeed`) :!via `PlayFromStart`)
    (:`Update`
      (bind _returnvalue (`KismetMathLibrary.Lerp` _radius (* _radius (`self.RadiusDemoMax`)) _newtrack_0))
      (`KismetMaterialLibrary.SetScalarParameterValue` "/Game/Vefects/Vertex_Collapse_VFX/VFX/Materials/Collections/MPC_Vefects_Vertex_Collapse_01.MPC_Vefects_Vertex_Collapse_01" "CollapseRadius" _returnvalue)
      (`SceneComponent.SetRelativeScale3D` (`self.SphereDebug`) (`KismetMathLibrary.Conv_DoubleToVector` (/ _returnvalue 100.0))))))

(fn `UserConstructionScript`
  (bind _spheredebug (`self.SphereDebug`))
  (`SceneComponent.K2_AddWorldOffset` (`self.SphereDebug`) (`self.PosOffset`) false false)
  (if (`self.activeDebug`)
    (`SceneComponent.SetHiddenInGame` _spheredebug false false)
    (`SceneComponent.SetVisibility` _spheredebug true false)
    (else
      (`SceneComponent.SetHiddenInGame` _spheredebug true false)
      (`SceneComponent.SetVisibility` _spheredebug false false))))